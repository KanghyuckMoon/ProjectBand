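; Song manager for a rhythm game that runs the flow from selection menu with random-position audio previews to gameplay and end screen.
; A chosen song's Level Sequence sets playback and length, feeding RhythmGamePawn lane creation along with lane data and auto or manual BPM.
; Sequence completion ends the round, while GameOver first ramps pitch through a timeline before stopping playback and showing score and max combo.
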(event Custom|ShowEndScreen
  (bind _rhythmgamepawn (Variables|Default|GetRhythmGamePawn))
  ;[1 1 1] Show score on the UI
  (bind _returnvalue (UserInterface|CreateWidget "/Game/BP/Blueprints/UI/BP_EndScreen.BP_EndScreen_C" 0 (Variables|/Game/BP/Blueprints/BP_RhythmGamePawn.BP_RhythmGamePawn_C|Getscore _rhythmgamepawn) (Variables|/Game/BP/Blueprints/BP_RhythmGamePawn.BP_RhythmGamePawn_C|GetmaxCombo _rhythmgamepawn) self))
  (bind _output_get (Variables|Default|SetendScreenUI _returnvalue))
  (Input|SetInputModeUIOnly (Game|GetPlayerController 0) _output_get "DoNotLock" false)
  (Variables|/Script/Engine.PlayerController|SetbShowMouseCursor (Game|GetPlayerController 0) true)
  (UserInterface|Viewport|AddtoViewport (Variables|Default|GetendScreenUI) 0))

(event Custom|PlayTheSong
  ;[1 1 1] Start the game and play the song
  (CallFunction|ResetPitchandVolume)
  (Sequencer|Player|Play (Variables|/Script/LevelSequence.LevelSequenceActor|GetSequencePlayer (Variables|Default|GetsequencePlayer)) :!class /Script/MovieScene.MovieSceneSequencePlayer)
  (Default|StartGame (Variables|Default|GetRhythmGamePawn)))

(event Custom|CreateSequencePlayer
  (bind _currentsong (Variables|Default|GetcurrentSong))
  (bind _songsequence (Utilities|Struct|BreakSongData _currentsong))
  ;[1 1 1] Create level sequence to play the song
  (Utilities|IsValid _songsequence
    (:Is%20Valid
      (bind (_outactor _returnvalue) (Sequencer|Player|CreateLevelSequencePlayer _songsequence))
      (Variables|Default|SetsequencePlayer _outactor)
      (EventDispatchers|AssignOnFinished _returnvalue (delegate Custom|OnFinishedHandler)))))

(event Custom|OnFinishedHandler
  ;[1 1 1] Create level sequence to play the song
  (EventDispatchers|UnbindEventfromOnFinished (stale Custom|CreateSequencePlayer _returnvalue) (delegate Custom|OnFinishedHandler))
  (if (not (Variables|Default|GetisGameOver))
    (Actor|DestroyActor (Variables|Default|GetsequencePlayer))
    (Default|OnGameOver (Variables|Default|GetRhythmGamePawn))
    (Variables|Default|SetisGameOver true)
    (CallFunction|ShowEndScreen)))

(event Custom|ResetPitchAndVolume
  ;[1 1 1] Reset pitch and volume of the song
  (Class|SongReader|SetSongVolume 1.0)
  (Class|SongReader|SetSongPitch 1.0))

(event Custom|StartPreviewSong
  (params (songData :type Song%20Data%20Structure))
  ;[1 1 1] Play random part of the song when mouse over
  (bind _returnvalue (Class|SongReader|GetSong songData))
  (Audio|Components|Audio|SetSound (Variables|Default|GetPreviewSongComponent) _returnvalue)
  (Audio|Components|Audio|Play (Variables|Default|GetPreviewSongComponent) (Math|Random|RandomFloatinRange 0.0 (- (Variables|/Script/Engine.SoundBase|GetDuration _returnvalue) 1e+01))))

(event Custom|StopPreviewSong
  ;[1 1 1] Stop playing song when mouse is not over the UI
  (Audio|Components|Audio|Stop (Variables|Default|GetPreviewSongComponent)))

(event Custom|OnSongChosen
  (params (songData :type Song%20Data%20Structure))
  (bind _returnvalue (Game|GetPlayerController 0))
  (bind _sequenceplayer (Variables|Default|GetsequencePlayer))
  (bind _sequenceplayer_2 (Variables|/Script/LevelSequence.LevelSequenceActor|GetSequencePlayer _sequenceplayer))
  (bind _returnvalue_2 (Media|MediaPlayer|GetDuration _sequenceplayer_2))
  (bind (_frame _framerate) (Utilities|TimeManagement|BreakQualifiedFrameTime _returnvalue_2))
  ;[1 1 1] Set song and create beats on the lane
  (Variables|Default|SetcurrentSong songData)
  (CallFunction|StopPreviewSong)
  (Widget|RemovefromParent (Variables|Default|GetsongSelectionMenu))
  (Input|SetInputModeGameOnly _returnvalue false)
  (Variables|/Script/Engine.PlayerController|SetbShowMouseCursor _returnvalue false)
  (Utilities|FlowControl|Delay 3.0)
  (CallFunction|CreateSequencePlayer)
  (bind _returnvalue_3 (Class|SongReader|GetLaneData (Variables|Default|GetcurrentSong)))
  (Default|CreateLanes (Variables|Default|GetRhythmGamePawn) self _returnvalue_3 (/ (Math|Conversions|ToFloat(Integer) (Utilities|Struct|BreakFrameNumber _frame)) (Math|Conversions|ToFloat(Integer) (.Numerator (Class|KismetMathLibrary|BreakFrameRate _framerate)))) (select (.autoCalculateBPM (Utilities|Struct|BreakSongData (Variables|Default|GetcurrentSong))) (Variables|Default|GetautoBPM) (.manualBPM (Utilities|Struct|BreakSongData (Variables|Default|GetcurrentSong)))))
  (CallFunction|PlaytheSong))

(event Custom|ShowSongSelectionMenu
  ;[1 1 1] Create list of songs on UI
  (Variables|Default|SetisGameOver false)
  (bind _returnvalue (UserInterface|CreateWidget "/Game/BP/Blueprints/UI/BP_SongSelectionMenu.BP_SongSelectionMenu_C" 0 (Variables|Default|GetlistOfSongs) self))
  (bind _output_get (Variables|Default|SetsongSelectionMenu _returnvalue))
  (UserInterface|Viewport|AddtoViewport _output_get 0)
  (Input|SetInputModeUIOnly (Game|GetPlayerController 0) (Variables|Default|GetsongSelectionMenu) "DoNotLock" false)
  (Variables|/Script/Engine.PlayerController|SetbShowMouseCursor (Game|GetPlayerController 0) true))

(event Custom|GameOver
  ;[1 1 1] Stop the song and destroy level sequencer
  (Variables|Default|SetisGameOver true)
  (Default|OnGameOver (Variables|Default|GetRhythmGamePawn))
  (Class|SongReader|SetSongVolume 1.0)
  (bind _pitch (Timeline|PitchOverTime PlayFromStart)
    (:Update
      (Class|SongReader|SetSongPitch _pitch))
    (:Finished
      (Sequencer|Player|Stop (Variables|/Script/LevelSequence.LevelSequenceActor|GetSequencePlayer (Variables|Default|GetsequencePlayer)) :!class /Script/MovieScene.MovieSceneSequencePlayer)
      (CallFunction|ResetPitchandVolume)
      (CallFunction|ShowEndScreen)
      (Actor|DestroyActor (Variables|Default|GetsequencePlayer)))))

(event EventBeginPlay
  ;[1 1 1] Show song selection UI
  (CallFunction|ShowSongSelectionMenu))

(fn ConstructionScript)