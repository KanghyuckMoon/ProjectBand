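; BP_Lane is one lane of a beat-based rhythm game, carrying beat actors as it scrolls along X.
; Initialize scales the spline's length by BPM, then spawns single and continuous beats from BeatData at time-based spline positions.
; Beats take the lane's indexed material and attach to it, so they travel with it.
; MoveTheLane lerps the actor toward the negated X of the spline's end through a timeline rate-scaled by SequenceLength.
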(event Custom|CreateBeatsOnTheLane
  (CallFunction|CreateSingleBeats)
  (CallFunction|CreateContinuousBeats))

(event Custom|MoveTheLane
  (bind _spline (Variables|Default|GetSpline))
  (bind _returnvalue (Spline|GetLocationatTime _spline 1.0 "World" false))
  (Variables|Default|SetlaneStartLocation (Transformation|GetActorLocation))
  (Variables|Default|SetlaneEndLocation (Math|Vector|MakeVector (* (.x _returnvalue) -1.0) (.y _returnvalue) (.z _returnvalue)))
  (Components|Timeline|SetPlayRate (Variables|Default|GetMoveOverTime) (/ 1.0 (Variables|Default|GetsequenceLength)))
  (bind _alpha (Timeline|MoveOverTime PlayFromStart)
    (:Update
      (Transformation|SetActorLocation (Math|Vector|Lerp(Vector) (Variables|Default|GetlaneStartLocation) (Variables|Default|GetlaneEndLocation) _alpha) false false))))

(event Custom|AdjustLaneLength
  (Spline|SetLocationatSplinePoint (Variables|Default|GetSpline) 1 (Math|Vector|MakeVector (* (Variables|Default|GetBPM) 7.0) 0.0 0.0) "Local" true))

(event Custom|Initialize
  (CallFunction|AdjustLaneLength)
  (CallFunction|CreateBeatsontheLane))

(event Custom|CreateSingleBeats
  (for _array_element (Utilities|Struct|BreakLaneData (Variables|Default|GetbeatData))
    (bind _returnvalue (Game|SpawnActorfromClass "/Game/BP/Blueprints/Beats/BP_SingleBeat.BP_SingleBeat_C" (Math|Conversions|ToTransform(Vector) (Spline|GetLocationatTime (Variables|Default|GetSpline) _array_element "World" false)) "Undefined" 0 (Utilities|Array|Get(acopy) (Variables|Default|GetlaneMatColors) (Variables|Default|GetlaneIndex)) self 0))
    (Transformation|AttachActorToActor _returnvalue self "None" "KeepWorld" "KeepWorld" "KeepWorld" true)))

(event Custom|CreateContinuousBeats
  (bind _spline (Variables|Default|GetSpline))
  (for _array_element (Utilities|Struct|BreakLaneData (Variables|Default|GetbeatData))
    (bind _returnvalue (Game|SpawnActorfromClass "/Game/BP/Blueprints/Beats/BP_ContinuousBeat.BP_ContinuousBeat_C" (Math|Conversions|ToTransform(Vector) (Spline|GetLocationatTime _spline (.startTime (Utilities|Struct|BreakContinuousBeat _array_element)) "World" false)) "Undefined" 0 (Spline|GetLocationatTime _spline (.startTime (Utilities|Struct|BreakContinuousBeat _array_element)) "World" false) (Spline|GetLocationatTime _spline (.endTime (Utilities|Struct|BreakContinuousBeat _array_element)) "World" false) (Utilities|Array|Get(acopy) (Variables|Default|GetlaneMatColors) (Variables|Default|GetlaneIndex)) self 0))
    (Transformation|AttachActorToActor _returnvalue self "None" "KeepWorld" "KeepWorld" "KeepWorld" true)))

(fn ConstructionScript)