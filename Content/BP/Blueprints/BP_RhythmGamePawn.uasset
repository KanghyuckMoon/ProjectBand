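; Player pawn for a rhythm game that runs the beat lanes, scoring and fail state.
; It spawns a lane at each child-actor beat player and forwards keyboard, mouse or mic clicks from the device input controller to matching players every tick.
; Hits build score and a combo-driven multiplier, mirroring results to the GameInstance and UI.
; Misses duck song volume, reset the combo and end the game through the SongReader after too many in a row.
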(event Custom|OnBeatPlayed
  ;[1 1 1] On beat played successfuly
  (Class|SongReader|SetSongVolume (Variables|Default|GetsongReader) 1.0)
  (Variables|Default|SetmissedBeatsInARow 0)
  (CallFunction|IncreaseScore 50)
  (CallFunction|IncreaseCombo)
  (bind _asbp_rhythm_game_game_instance (Utilities|Casting|CastToBP_RhythmGameGameInstance (Game|GetGameInstance)))
  (Variables|/Game/BP/Blueprints/BP_RhythmGameGameInstance.BP_RhythmGameGameInstance_C|SetSuccessNodeCount _asbp_rhythm_game_game_instance (+ (Variables|/Game/BP/Blueprints/BP_RhythmGameGameInstance.BP_RhythmGameGameInstance_C|GetSuccessNodeCount _asbp_rhythm_game_game_instance) 1)))

(event Custom|CreateLanes
  (params (songReader :type BP%20Song%20Reader%20Object%20Reference) (laneData :type Array%20of%20Lane%20Data%20Structures) (sequenceLength :type Float%20%28double-precision%29) (BPM :type Float%20%28double-precision%29))
  ;[1 1 1] Create lanes
  (bind _asbp_rhythm_game_game_instance (Utilities|Casting|CastToBP_RhythmGameGameInstance (Game|GetGameInstance)))
  (Variables|/Game/BP/Blueprints/BP_RhythmGameGameInstance.BP_RhythmGameGameInstance_C|SetFullNodeCount _asbp_rhythm_game_game_instance 0)
  (Variables|Default|SetsongReader songReader)
  (Utilities|Array|Clear (Variables|Default|Getlanes))
  (CallFunction|CreateGameUI)
  (CallFunction|StoreAllBeatPlayers)
  (for (_array_element _array_index) laneData
    (bind _asbp_rhythm_game_game_instance_2 (Utilities|Casting|CastToBP_RhythmGameGameInstance (Game|GetGameInstance)))
    (bind _output_get (Variables|/Game/BP/Blueprints/BP_RhythmGameGameInstance.BP_RhythmGameGameInstance_C|SetFullNodeCount _asbp_rhythm_game_game_instance_2 (+ (Utilities|Array|Length (.listOfSingleBeats (Utilities|Struct|BreakLaneData _array_element))) (Variables|/Game/BP/Blueprints/BP_RhythmGameGameInstance.BP_RhythmGameGameInstance_C|GetFullNodeCount _asbp_rhythm_game_game_instance_2))))
    (Development|PrintString (Utilities|String|ToString(Integer) _output_get))
    (if (<= _array_index (Utilities|Array|LastIndex (Variables|Default|GetbeatPlayers)))
      (bind _returnvalue (Game|SpawnActorfromClass "/Game/BP/Blueprints/BP_Lane.BP_Lane_C" (Math|Conversions|ToTransform(Vector) (Transformation|GetActorLocation (Utilities|Array|Get(acopy) (Variables|Default|GetbeatPlayers) _array_index))) "Undefined" 0 _array_element sequenceLength BPM _array_index 0))
      (Default|Initialize _returnvalue)
      (Utilities|Array|Add (Variables|Default|Getlanes) _returnvalue))))

(event Custom|ResetCombo
  ;[1 1 1] Score calculation
  (bind _output_get (Variables|Default|Setcombo 0))
  (Default|UpdateCombo (Variables|Default|GetgameUI) _output_get)
  (CallFunction|CalculateMultiplier))

(event Custom|CalculateMultiplier
  ;[1 1 1] Score calculation
  (Variables|Default|SetscoreMultiplier (Math|Integer|Clamp(Integer) (+ (.ReturnValue (Math|Float|Division(WholeandRemainder) (Math|Conversions|ToFloat(Integer) (Variables|Default|Getcombo)) 1e+01)) 1) 1 5))
  (CallFunction|CalculateComboCounter))

(event Custom|CalculateComboCounter
  (bind _combo (Variables|Default|Getcombo))
  (bind _returnvalue (Math|Conversions|ToFloat(Integer) _combo))
  (bind (_remainder _returnvalue_2) (Math|Float|Division(WholeandRemainder) _returnvalue 1e+01))
  ;[1 1 1] Score calculation
  (if (or (!= _remainder 0.0) (== _returnvalue_2 0))
    _))

(event Custom|ResetScore
  ;[1 1 1] Score calculation
  (bind _output_get (Variables|Default|Setscore 0))
  (Default|UpdateScore (Variables|Default|GetgameUI) _output_get)
  (Variables|Default|SetscoreMultiplier 1)
  (CallFunction|ResetCombo))

(event Custom|StartGame
  ;[1 1 1] Reset score and start the game
  (CallFunction|ResetScore)
  (Variables|Default|SetmissedBeatsInARow 0)
  (Variables|Default|SetmaxCombo 0)
  (for _array_element (Variables|Default|Getlanes)
    (Default|MovetheLane _array_element)
    (bind _asbp_rhythm_game_game_instance (Utilities|Casting|CastToBP_RhythmGameGameInstance (Game|GetGameInstance)))
    (Variables|/Game/BP/Blueprints/BP_RhythmGameGameInstance.BP_RhythmGameGameInstance_C|SetScore _asbp_rhythm_game_game_instance 0)
    (Variables|/Game/BP/Blueprints/BP_RhythmGameGameInstance.BP_RhythmGameGameInstance_C|SetSuccessNodeCount _asbp_rhythm_game_game_instance 0)
    (bind _asbp_beat_player (Utilities|Casting|CastToBP_BeatPlayer (Variables|/Script/Engine.ChildActorComponent|GetChildActor (Variables|Default|Get1LaneBeatPlayer))))
    (Variables|/Game/BP/Blueprints/BP_BeatPlayer.BP_BeatPlayer_C|SetIsGuitar _asbp_beat_player true)
    (bind _asbp_beat_player_2 (Utilities|Casting|CastToBP_BeatPlayer (Variables|/Script/Engine.ChildActorComponent|GetChildActor (Variables|Default|Get2LaneBeatPlayer))))
    (Variables|/Game/BP/Blueprints/BP_BeatPlayer.BP_BeatPlayer_C|SetIsGuitar _asbp_beat_player_2 false)))

(event Custom|StoreAllBeatPlayers
  ;[1 1 1] Initialize the beat players
  (Utilities|Array|Clear (Variables|Default|GetbeatPlayers))
  (for _array_element (Utilities|Array|MakeArray (Variables|Default|Get1LaneBeatPlayer) (Variables|Default|Get2LaneBeatPlayer) (Variables|Default|Get3LaneBeatPlayer) 0 0)
    (bind _asbp_beat_player (Utilities|Casting|CastToBP_BeatPlayer (Variables|/Script/Engine.ChildActorComponent|GetChildActor _array_element)))
    (Default|Initialize _asbp_beat_player self)
    (Utilities|Array|Add (Variables|Default|GetbeatPlayers) _asbp_beat_player)))

(event Custom|OnBeatMissed
  ;[1 1 1] On failed to play beat
  (Class|SongReader|SetSongVolume (Variables|Default|GetsongReader) 0.25)
  (CallFunction|ResetCombo)
  (bind _result (Math|Integer|IncrementInt (Variables|Default|GetmissedBeatsInARow))
    (:%20%20
      (if (and (>= _result (Variables|Default|GetmistakesInARowToGameOver)) (not (Variables|/Game/BP/Blueprints/BP_SongReader.BP_SongReader_C|GetisGameOver (Variables|Default|GetsongReader))))
        (Default|GameOver (Variables|Default|GetsongReader))))))

(event Custom|OnWrongBeat
  ;[1 1 1] On failed to play beat
)

(event Custom|OnGameOver
  ;[1 1 1] Destory lanes on game over
  (Widget|RemovefromParent (Variables|Default|GetgameUI))
  (bind _arrayelement (Utilities|Array|ReverseforEachLoop (Variables|Default|Getlanes))
    (:LoopBody
      (Utilities|IsValid _arrayelement
        (:Is%20Valid
          (Actor|DestroyActor _arrayelement))))))

(event Custom|CreateGameUI
  ;[1 1 1] Show game UI
  (bind _returnvalue (UserInterface|CreateWidget "/Game/BP/Blueprints/UI/BP_GameUI.BP_GameUI_C"))
  (bind _output_get (Variables|Default|SetgameUI _returnvalue))
  (UserInterface|Viewport|AddtoViewport _output_get 0))

(event Custom|IncreaseScore
  (params (scoreToAdd :type Integer))
  ;[1 1 1] Score calculation
  (bind _output_get (Variables|Default|Setscore (+ (Variables|Default|Getscore) (* scoreToAdd (Variables|Default|GetscoreMultiplier)))))
  (Default|UpdateScore (Variables|Default|GetgameUI) _output_get)
  (bind _asbp_rhythm_game_game_instance (Utilities|Casting|CastToBP_RhythmGameGameInstance (Game|GetGameInstance)))
  (Variables|/Game/BP/Blueprints/BP_RhythmGameGameInstance.BP_RhythmGameGameInstance_C|SetScore _asbp_rhythm_game_game_instance _output_get))

(event Custom|IncreaseCombo
  ;[1 1 1] Score calculation
  (bind _result (Math|Integer|IncrementInt (Variables|Default|Getcombo))
    (:%20%20
      (Default|UpdateCombo (Variables|Default|GetgameUI) _result)
      (CallFunction|CalculateMultiplier)
      (Variables|Default|SetmaxCombo (Math|Integer|Max(Integer) (Variables|Default|Getcombo) (Variables|Default|GetmaxCombo))))))

(event EventTick
  (params (DeltaSeconds :type Float%20%28single-precision%29))
  (bind _asbp_device_input_controller (Utilities|Casting|CastToBP_DeviceInputController (Game|GetPlayerController 0)))
  ;[1 1 1] Detect player input
  (if (or (or (Variables|/Script/ProjectBand.DeviceInputController|GetisClickKeyboard _asbp_device_input_controller) (Variables|/Script/ProjectBand.DeviceInputController|GetisClickMouse _asbp_device_input_controller)) (or (Variables|/Script/ProjectBand.DeviceInputController|GetisClickMouse _asbp_device_input_controller) (Variables|/Script/ProjectBand.DeviceInputController|GetisClickMike _asbp_device_input_controller)))
    (Variables|Default|SetkeyPressed true)
    (else
      (Variables|Default|SetkeyPressed false)))
  (for _array_element (Variables|Default|GetbeatPlayers)
    (switch Utilities|FlowControl|Switch|SwitchonInputType (Variables|/Game/BP/Blueprints/BP_BeatPlayer.BP_BeatPlayer_C|GetInputType _array_element)
      (:NewEnumerator0
        (if (Variables|/Script/ProjectBand.DeviceInputController|GetisClickKeyboard _asbp_device_input_controller)
          (Default|KeyInput _array_element (Variables|Default|GetkeyPressed) :!label _label)
          (else
            (Default|KeyInput _array_element false :!label _label_2))))
      (:NewEnumerator1
        (if (Variables|/Script/ProjectBand.DeviceInputController|GetisClickMouse _asbp_device_input_controller)
          (goto _label)
          (else
            (goto _label_2))))
      (:NewEnumerator2
        (if (Variables|/Script/ProjectBand.DeviceInputController|GetisClickMike _asbp_device_input_controller)
          (goto _label)
          (else
            (goto _label_2)))))))

(fn ConstructionScript)

(fn SetKeyBoardDelay
  (params (Delay :type Float%20%28double-precision%29))
  (bind _asbp_beat_player (Utilities|Casting|CastToBP_BeatPlayer (Variables|/Script/Engine.ChildActorComponent|GetChildActor (Variables|Default|Get1LaneBeatPlayer))))
  (Default|SetLaneDelay _asbp_beat_player Delay))

(fn SetMouseDelay
  (params (Delay :type Float%20%28double-precision%29))
  (bind _asbp_beat_player (Utilities|Casting|CastToBP_BeatPlayer (Variables|/Script/Engine.ChildActorComponent|GetChildActor (Variables|Default|Get2LaneBeatPlayer))))
  (Default|SetLaneDelay _asbp_beat_player Delay))

(fn SetMikeDelay
  (params (Delay :type Float%20%28double-precision%29))
  (bind _asbp_beat_player (Utilities|Casting|CastToBP_BeatPlayer (Variables|/Script/Engine.ChildActorComponent|GetChildActor (Variables|Default|Get3LaneBeatPlayer))))
  (Default|SetLaneDelay _asbp_beat_player Delay))