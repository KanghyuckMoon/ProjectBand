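; Continuous (held) beat for a lane-based rhythm mechanic, drawn as a line stretching from the beat to its end location.
; On BeginPlay it moves the end detector to that location, extends the spline there, and builds spline mesh segments attached to the lane root.
; Each segment gets a dynamic material, so a played beat drops its head mesh and glows, while a missed one is flagged and turns grey and unlit.
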(event Custom|AdjustBeatLength
  ;[1 1 1] Create spline and add mesh component to it
  (Transformation|SetWorldLocation (Variables|Default|GetBeatEndDetector) (Variables|Default|GetbeatEndLocation) false false)
  (Spline|AddSplinePoint (Variables|Default|GetSpline) (Variables|Default|GetbeatEndLocation) "World" true)
  (for _index (range 0 (- (Spline|GetNumberOfSplinePoints (Variables|Default|GetSpline)) 2))
    (bind _returnvalue (AddComponent|AddSplineMeshComponent true (Transformation|GetWorldTransform (Variables|Default|GetSpline))))
    (Transformation|SetMobility _returnvalue "Movable")
    (Transformation|AttachComponentToComponent _returnvalue (Variables|/Game/BP/Blueprints/BP_Lane.BP_Lane_C|GetDefaultSceneRoot (Variables|Default|Getlane)) "None" "KeepWorld" "KeepWorld" "KeepWorld" true)
    (Rendering|Material|SetMaterial _returnvalue 0 (Variables|Default|GetbeatMaterial))
    (bind _returnvalue_2 (Rendering|Material|CreateDynamicMaterialInstance _returnvalue 0 (Rendering|Material|GetMaterial _returnvalue 0) "None" :!class /Script/Engine.PrimitiveComponent))
    (Utilities|Array|Add (Variables|Default|GetdynamicMaterials) _returnvalue_2)
    (Utilities|Array|Add (Variables|Default|GetsplineMeshes) _returnvalue)
    (SplineMesh|SetStartandEnd _returnvalue (.Location (Spline|GetLocationandTangentatSplinePoint (Variables|Default|GetSpline) _index "Local")) (.Tangent (Spline|GetLocationandTangentatSplinePoint (Variables|Default|GetSpline) _index "Local")) (.Location (Spline|GetLocationandTangentatSplinePoint (Variables|Default|GetSpline) (+ _index 1) "Local")) (.Tangent (Spline|GetLocationandTangentatSplinePoint (Variables|Default|GetSpline) (+ _index 1) "Local")) true :!class /Script/Engine.SplineMeshComponent)))

(event Custom|IncreaseEmissivity
  ;[1 1 1] Glow the continuous beat line
  (for _array_element (Variables|Default|GetdynamicMaterials)
    (Rendering|Material|SetScalarParameterValue _array_element "Emissivity" 5e+01 :!class /Script/Engine.MaterialInstanceDynamic)))

(event EventBeginPlay
  ;[1 1 1] Adjust the continuous beat length
  (|CallParentFunction)
  (CallFunction|AdjustBeatLength))

(event EventOnBeatMissed
  ;[1 1 1] On failed to play continuous beat
  (Variables|Default|SetisMissed true)
  (for _array_element (Variables|Default|GetdynamicMaterials)
    (Rendering|Material|SetVectorParameterValue _array_element "Color" "(R=0.566406,G=0.566406,B=0.566406,A=1.000000)" :!class /Script/Engine.MaterialInstanceDynamic)
    (Rendering|Material|SetScalarParameterValue _array_element "Emissivity" 0.0 :!class /Script/Engine.MaterialInstanceDynamic)))

(event EventOnBeatPlayed
  ;[1 1 1] Destyor the beat mesh and glow on played
  (Components|DestroyComponent (Variables|Default|GetBeatMesh))
  (CallFunction|IncreaseEmissivity))

(fn ConstructionScript
  (|CallParentFunction))