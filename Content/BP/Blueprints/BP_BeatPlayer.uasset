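; BP_BeatPlayer is a rhythm game lane hit zone that turns touch or key input into beat hits.
; Presses brighten its decal, play overlapping BP_Beats and open a Tick gate that adds score to RhythmGamePawn.
; Release closes the gate, lowering song volume and missing any held beat.
; MissDetector flags passed beats and ends continuous ones, while input type and SetLaneDelay adjust detector geometry.
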(event OnInputTouchBegin(TouchDetector)
  (params (FingerIndex :type ETouchIndex%20Enum :default "Touch1") (TouchedComponent :type Primitive%20Component%20Object%20Reference))
  ;[1 1 1] Detect input press and release
  (CallFunction|KeyPressed))

(event OnComponentBeginOverlap(MissDetector)
  (params (OverlappedComponent :type Primitive%20Component%20Object%20Reference) (OtherActor :type Actor%20Object%20Reference) (OtherComp :type Primitive%20Component%20Object%20Reference) (OtherBodyIndex :type Integer) (bFromSweep :type Boolean) (SweepResult :type Hit%20Result%20Structure%20%28by%20ref%29))
  ;[1 1 1] Detect beat miss
  (bind _asbp_beat (Utilities|Casting|CastToBP_Beat OtherActor)
    (:then
      (Default|OnBeatMissed _asbp_beat)
      (Rendering|SetVisibility (Variables|Components|GetMissText) true false)
      (Default|OnBeatMissed (Variables|Actor|GetrhythmGamePawn))
      (Utilities|FlowControl|RetriggerableDelay 0.5)
      (Rendering|SetVisibility (Variables|Components|GetMissText) false false))
    (:CastFailed
      (Utilities|Casting|CastToBP_ContinuousBeatEnd OtherActor)
      (CallFunction|ContinuousScoreStop)
      (Variables|Actor|SetcurrentlyPlayingBeat 0))))

(event OnInputTouchEnd(TouchDetector)
  (params (FingerIndex :type ETouchIndex%20Enum :default "Touch1") (TouchedComponent :type Primitive%20Component%20Object%20Reference))
  ;[1 1 1] Detect input press and release
  (CallFunction|KeyReleased))

(event Custom|KeyInput
  (params (pressed :type Boolean))
  ;[1 1 1] Detect input press and release
  (if pressed
    (CallFunction|KeyPressed)
    (else
      (CallFunction|KeyReleased))))

(event Custom|KeyPressed
  ;[1 1 1] Start / stop playing beat
  (Rendering|Material|SetScalarParameterValue (Variables|Actor|GetdynamicMat) "Emissivity" 1e+02 :!class /Script/Engine.MaterialInstanceDynamic)
  (CallFunction|PlayBeat))

(event Custom|KeyReleased
  ;[1 1 1] Start / stop playing beat
  (Rendering|Material|SetScalarParameterValue (Variables|Actor|GetdynamicMat) "Emissivity" 1.0 :!class /Script/Engine.MaterialInstanceDynamic)
  (CallFunction|StopPlayingBeat))

(event Custom|PlayBeat
  (bind _touchdetector (Variables|Components|GetTouchDetector))
  (bind _overlappingactors (Collision|GetOverlappingActors _touchdetector "/Game/BP/Blueprints/Beats/BP_Beat.BP_Beat_C" :!class /Script/Engine.PrimitiveComponent))
  ;[1 1 1] Start playing beat
  (if (!= (Utilities|Array|Length _overlappingactors) 0)
    (Default|OnBeatPlayed (Variables|Actor|GetrhythmGamePawn))
    (for _array_element _overlappingactors
      (bind _asbp_beat (Utilities|Casting|CastToBP_Beat _array_element))
      (bind _output_get (Variables|Actor|SetcurrentlyPlayingBeat _asbp_beat))
      (Default|OnBeatPlayed _output_get)
      (Components|Activation|Activate (Variables|Components|GetSingleBeatParticle) true)
      (CallFunction|ContinuousScoreStart))))

(event Custom|Initialize
  (params (rhythmGamePawn :type BP%20Rhythm%20Game%20Pawn%20Object%20Reference))
  ;[1 1 1] Save pawn reference
  (Variables|Actor|SetrhythmGamePawn rhythmGamePawn))

(event Custom|StopPlayingBeat
  ;[1 1 1] Stop playing beat
  (CallFunction|ContinuousScoreStop)
  (Utilities|IsValid (Variables|Actor|GetcurrentlyPlayingBeat)
    (:Is%20Valid
      (Class|SongReader|SetSongVolume (Variables|/Game/BP/Blueprints/BP_RhythmGamePawn.BP_RhythmGamePawn_C|GetsongReader (Variables|Actor|GetrhythmGamePawn)) 0.25)
      (Default|OnBeatMissed (Variables|Actor|GetcurrentlyPlayingBeat))
      (Variables|Actor|SetcurrentlyPlayingBeat 0))))

(event Custom|ContinuousScoreStart
  ;[1 1 1] Play continuous beat
  (Utilities|IsValid (Variables|Actor|GetcurrentlyPlayingBeat)
    (:Is%20Valid
      (Utilities|FlowControl|Gate true) ; enters at Open
    )))

(event Custom|ContinuousScoreStop
  ;[1 1 1] Play continuous beat
  (Utilities|FlowControl|Gate true) ; enters at Close
)

(event EventBeginPlay
  (bind _touchdetector (Variables|Components|GetTouchDetector))
  ;[1 1 1] Create dynamic material
  (bind _returnvalue (Rendering|Material|CreateDynamicMaterialInstance (Variables|Components|GetBeatPlayerMat) :!class /Script/Engine.DecalComponent))
  (Variables|Actor|SetdynamicMat _returnvalue)
  (switch Utilities|FlowControl|Switch|SwitchonInputType (Variables|Default|GetInputType)
    (:NewEnumerator0
      (Transformation|SetRelativeLocation _touchdetector "0, 0, 0" false false)
      (Transformation|SetRelativeScale3D _touchdetector "2.000000,1.000000,1.000000"))
    (:NewEnumerator1
      (Transformation|SetRelativeLocation _touchdetector "0, 0, 0" false false)
      (Transformation|SetRelativeScale3D _touchdetector "2.000000,1.000000,1.000000"))
    (:NewEnumerator2
      (Transformation|SetRelativeLocation _touchdetector "-0.500000,0.000000,0.000000" false false)
      (Transformation|SetRelativeScale3D _touchdetector "3.000000,1.000000,1.000000")
      (Development|PrintString "Hello"))))

(event EventTick
  (params (DeltaSeconds :type Float%20%28single-precision%29))
  ;[1 1 1] Play continuous beat
  (Utilities|FlowControl|Gate true
    (:Exit
      (Utilities|FlowControl|Delay 0.1)
      (Default|IncreaseScore (Variables|Actor|GetrhythmGamePawn) 1)
      (Components|Activation|Activate (Variables|Components|GetContinuousBeatParticle) true))))

(fn ConstructionScript
  (Rendering|Components|Decal|SetDecalMaterial (Variables|Components|GetBeatPlayerMat) (Variables|Default|GetbeatPlayerMaterial)))

(fn SetLaneDelay
  (params (Delay :type Float%20%28double-precision%29))
  (Transformation|SetRelativeScale3D (Variables|Components|GetTouchDetector) (Math|Vector|MakeVector (+ Delay 1.0) 1.0 1.0))
  (Transformation|SetRelativeLocation (Variables|Components|GetMissDetector) (Math|Vector|MakeVector (- (* Delay -1e+01) -2e+01) 1.0 1.0) false false))